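; EnemySpawner is an actor that spawns a set of enemies for the player's current encounter when play begins.
; It reads EnemyEncounter from BP_PlayerController to pick an entry in EnemyPatterns.
; Each class in that pattern spawns at the EnemyLocations transform with the same index.
; A next-tick delay follows each spawn call in the loop, and an author note marks the logic as not working.
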(event EventBeginPlay
  (bind _asbp_player_controller (Utilities|Casting|CastToBP_PlayerController (Game|GetPlayerController 0))) ; don't work :(
  (for (_array_element _array_index) (Variables|/Game/Blueprints/Enemies/EnemyPatterns/PD_EnemyPatternBase.PD_EnemyPatternBase_C|GetEnemyPattern (Utilities|Array|Get(acopy) (Variables|Default|GetEnemyPatterns) (Variables|/Game/Blueprints/Player/BP_PlayerController.BP_PlayerController_C|GetEnemyEncounter _asbp_player_controller)))
    (Game|SpawnActorfromClass _array_element (Utilities|Array|Get(acopy) (Variables|Default|GetEnemyLocations) _array_index) "Undefined" "MultiplyWithRoot" 0 0)
    (Utilities|FlowControl|DelayUntilNextTick)))

(event Collision|EventActorBeginOverlap
  (params (OtherActor :type Actor%20Object%20Reference)))

(fn ConstructionScript)
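; Base enemy for combat that repeatedly damages a player's health component on a Speed-based delay, with a timeline cube lunge.
; Tick drives attacks through placeholder targeting that indexes combat players, advances past dead ones and prints game over when the index runs out.
; Health component events flash the cube red on damage and destroy the actor on death.
; A targeted event briefly shows an indicator plane.
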(event OnDeath(AC_HealthComponent)
  ;[0.15 0.15 0.15 0.5] Enemy dies if on death is recieved
  (Development|PrintString "Enemy dead")
  (Actor|DestroyActor))

(event OnDamaged(AC_HealthComponent)
  (params (DamageTaken :type Float%20%28double-precision%29))
  (bind _cube (Variables|Default|GetCube))
  ;[0.15 0.15 0.15 0.5] Makes red when taking damage
  (Rendering|Material|SetMaterial _cube 0 "/Game/Material/M_Red.M_Red")
  (Utilities|FlowControl|Delay 0.5)
  (Rendering|Material|SetMaterial _cube 0 "/Game/Material/M_White.M_White"))

(event Custom|OnTargetted_Event
  (bind _targettedplane (Variables|Default|GetTargettedPlane))
  (Rendering|SetVisibility _targettedplane true false)
  (Utilities|FlowControl|Delay 0.4)
  (Rendering|SetVisibility _targettedplane false false))

(event EventBeginPlay
  ;[0.15 0.15 0.15 0.5] Init
  (Variables|Default|SetStartPos (Transformation|GetWorldTransform (Variables|Default|GetCube)))
  (CallFunction|TargetPlayer)
  (EventDispatchers|BindEventtoOnTargetted (delegate Custom|OnTargetted_Event)))

(event EventTick
  (params (DeltaSeconds :type Float%20%28single-precision%29))
  ;[0.15 0.15 0.15 0.5] Attacks Player
  (if (Variables|Default|GetCanAttack)
    (CallFunction|TargetPlayer)
    (Default|TakeDamage (Variables|Default|GetTarget) (Variables|Default|GetAttackDamage))
    (Variables|Default|SetCanAttack false)
    ;[0.15 0.15 0.15 0.5] Animate attack
    (bind _alpha (Timeline|AttackAnimTimeline PlayFromStart)
      (:Update
        (Transformation|SetWorldTransform (Variables|Default|GetCube) (Math|Interpolation|Ease "Linear" _alpha (Variables|Default|GetStartPos) (Math|Conversions|ToTransform(Vector) (+ (.location (Variables|Default|GetStartPos)) "0.000000,50.000000,0.000000"))) false false)))
    (else
      (Utilities|FlowControl|Delay (* (Variables|Default|GetSpeed) 1.0))
      (Variables|Default|SetCanAttack true))))

(fn ConstructionScript)

(fn TargetPlayer
  (bind _currenttarget (Variables|Default|GetCurrentTarget))
  ;[0.15 0.15 0.15 0.5] Placeholder targeting
  (bind _outactors (Actor|GetAllActorsOfClass "/Game/Blueprints/Player/BP_CombatPlayerBase.BP_CombatPlayerBase_C"))
  (bind _asbp_combat_player_base (Utilities|Casting|CastToBP_CombatPlayerBase (Utilities|Array|Get(acopy) _outactors (Variables|Default|GetCurrentTarget))))
  (if (Variables|/Game/Blueprints/Player/BP_CombatPlayerBase.BP_CombatPlayerBase_C|GetIsDead _asbp_combat_player_base)
    (Utilities|Array|RemoveIndex _outactors _currenttarget)
    (bind _result (Math|Integer|IncrementInt _currenttarget)
      (:%20%20
        (if (not (Utilities|Array|IsValidIndex _outactors (Math|Integer|Clamp(Integer) _result 0 (Utilities|Array|Length _outactors))))
          (Development|PrintString "game over"))))
    (else
      (Variables|Default|SetTarget (Variables|/Game/Blueprints/Player/BP_CombatPlayerBase.BP_CombatPlayerBase_C|GetAC_HealthComponent _asbp_combat_player_base)))))
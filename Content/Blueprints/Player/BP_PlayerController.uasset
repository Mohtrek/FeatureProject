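; Player controller that records movement input and offers a debug shortcut into combat.
; IA_Move writes its axes, with X and Y swapped, into a normalized MoveDir vector and zeroes it on release.
; The M debug key opens the Combat level.
; Unconnected draft nodes sketch a level-name check and swapping the possessed pawn between combat and overworld player classes, but never run.
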(event Input|EnhancedActionEvents|EnhancedInputActionIA_Move
  (params (ActionValue :type Vector%202D%20Structure) (ElapsedSeconds :type Float%20%28double-precision%29) (TriggeredSeconds :type Float%20%28double-precision%29) (InputAction :type Input%20Action%20Object%20Reference :default "/Game/Inputs/InputActions/IA_Move.IA_Move"))
  ;[0.15 0.15 0.15 0.5] Set player move direction
  (:Triggered
    (bind _output_get (Variables|Default|SetMoveDir (Math|Vector|MakeVector (.y ActionValue) (.x ActionValue) 0.0)))
    (Variables|Default|SetMoveDir (Math|Vector|Normalize _output_get)))
  (:Completed
    (Variables|Default|SetMoveDir "0, 0, 0")))

(event EventBeginPlay)

(event Input|KeyboardEvents|DebugKeyM
  (params (Key :type Key%20Structure :default "None") (ActionValue :type Input%20Action%20Value%20Structure))
  (:Pressed
    (Game|OpenLevel(byObjectReference) "/Game/Levels/Combat.Combat")))

(fn ConstructionScript)
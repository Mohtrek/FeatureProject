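; Overworld player that moves around the map and carries a debug shortcut into combat.
; On BeginPlay it caches BP_PlayerController and adds the IMC_Inputs Enhanced Input mapping context.
; Each Tick sweeps its Cube component along the controller's MoveDir, scaled by MoveSpeed and delta time.
; Debug key M sets the game mode's default pawn to BP_CombatPlayerBase and loads Combat as a level instance.
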(event EventBeginPlay
  ;[0.15 0.15 0.15 0.5] Get Input system
  (bind _asbp_player_controller (Utilities|Casting|CastToBP_PlayerController (Game|GetPlayerController 0)))
  (Variables|Default|SetPlayer%20Controller _asbp_player_controller)
  (bind _asplayer_controller (Utilities|Casting|CastToPlayerController (Pawn|GetController)))
  (Utilities|IsValid (PlayerController|LocalPlayerSubsystems|GetEnhancedInputLocalPlayerSubsystem _asplayer_controller)
    (:Is%20Valid
      (Input|AddMappingContext (PlayerController|LocalPlayerSubsystems|GetEnhancedInputLocalPlayerSubsystem _asplayer_controller) "/Game/Inputs/IMC_Inputs.IMC_Inputs" 0 "(bIgnoreAllPressedKeysUntilRelease=True,bForceImmediately=False,bNotifyUserSettings=False)"))))

(event EventTick
  (params (DeltaSeconds :type Float%20%28single-precision%29))
  ;[0.15 0.15 0.15 0.5] Moves Player
  (Transformation|AddWorldOffset (Variables|Default|GetCube) (* DeltaSeconds (Variables|/Game/Blueprints/Player/BP_PlayerController.BP_PlayerController_C|GetMoveDir (Variables|Default|GetPlayer%20Controller)) (Variables|Default|GetMoveSpeed)) true false))

(event Collision|EventActorBeginOverlap
  (params (OtherActor :type Actor%20Object%20Reference)))

(event Input|KeyboardEvents|DebugKeyM
  (params (Key :type Key%20Structure :default "None") (ActionValue :type Input%20Action%20Value%20Structure))
  (:Pressed
    (bind _asbp_game_mode (Utilities|Casting|CastToBP_GameMode (Game|GetGameMode)))
    (Variables|/Script/Engine.GameModeBase|SetDefaultPawnClass _asbp_game_mode "/Game/Blueprints/Player/BP_CombatPlayerBase.BP_CombatPlayerBase_C")
    (Class|LevelStreamingDynamic|LoadLevelInstancebySoftObjectPtr "/Game/Levels/Combat.Combat" "0, 0, 0" "0, 0, 0" "" 0 false)))

(fn ConstructionScript)